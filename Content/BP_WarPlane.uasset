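; War plane Blueprint that sets up the player's on-screen interface, with flight steering present but not connected.
; BeginPlay adds an EngineInformation widget to the viewport and shows the mouse cursor, while Tick only prints the frame delta time.
; An unconnected chain would raise pitch toward a 60-degree limit when the cursor is in the upper screen half, faster nearer the top, switching to a variable step at the edge.
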(event EventBeginPlay
  (bind _returnvalue (UserInterface|CreateWidget "/Game/EngineInformation.EngineInformation_C"))
  (UserInterface|Viewport|AddtoViewport _returnvalue 0)
  (Variables|/Script/Engine.PlayerController|SetbShowMouseCursor (Game|GetPlayerController 0) true))

(event EventTick
  (params (DeltaSeconds :type Float%20%28single-precision%29))
  (Development|PrintString (Utilities|String|ToString(Float) DeltaSeconds)))

(fn ConstructionScript)